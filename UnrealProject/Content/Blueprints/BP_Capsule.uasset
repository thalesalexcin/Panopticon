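; BP_Capsule is an actor that floats its Sphere component and destroys itself based on game and alert state.
; Each tick it destroys itself if PanoGameMode leaves two allowed states or its AlertActor reaches a specific warning state.
; It also advances a timer and applies transform-corrected local offsets from per-axis sine helpers, with separate speeds and shared amplitude.
; The helpers' sine-difference expressions appear unconnected to any output.
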(event `self.ReceiveTick`
  (params (DeltaSeconds :type "Float (single-precision)"))
  (`|ExecutionSequence`
    (:`then_0`
      (bind _aspano_game_mode (cast `/Game/Blueprints/PanoGameMode` (`GameplayStatics.GetGameMode`)))
      (bind _currentgamestate (`/Game/Blueprints/PanoGameMode.CurrentGameState` _aspano_game_mode))
      (if (or (`|EnumEquality` _currentgamestate "NewEnumerator1") (`|EnumEquality` _currentgamestate "NewEnumerator2"))
        (if (`|EnumEquality` (`/Game/Blueprints/BP_AlertActor.CurrentWarningState` (`self.AlertActor`)) "NewEnumerator3")
          (`self.K2_DestroyActor` :!label _label))
        (else
          (goto _label))))
    (:`then_1`
      (set `self.Timer` (+ (`self.Timer`) DeltaSeconds)))
    (:`then_2`
      (`self.Floating effect` DeltaSeconds))))

(fn `Floating effect`
  (params (DeltaTime :type "Float (double-precision)"))
  (bind _sphere (`self.Sphere`))
  (bind _floatingamplitude (`self.FloatingAmplitude`))
  (bind _returnvalue (* (`self.Timer`) (`self.FloatingSpeed_Y`)))
  (bind _returnvalue_2 (* (`self.Timer`) (`self.FloatingSpeed_Z`)))
  (bind _returnvalue_3 (* (`self.Timer`) (`self.FloatingSpeed_X`)))
  (`SceneComponent.K2_AddLocalOffset` _sphere (`KismetMathLibrary.InverseTransformDirection` (`SceneComponent.GetRelativeTransform` _sphere) (`KismetMathLibrary.MakeVector` (* (- (`KismetMathLibrary.Sin` (+ DeltaTime _returnvalue_3)) (`KismetMathLibrary.Sin` _returnvalue_3)) _floatingamplitude) (* (- (`KismetMathLibrary.Sin` (+ DeltaTime _returnvalue)) (`KismetMathLibrary.Sin` _returnvalue)) _floatingamplitude) (* (- (`KismetMathLibrary.Sin` (+ DeltaTime _returnvalue_2)) (`KismetMathLibrary.Sin` _returnvalue_2)) _floatingamplitude))) false false)
  (return))

(fn `UserConstructionScript`)