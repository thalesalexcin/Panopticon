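; ID panel actor where the player judges an alert profile as suspect or innocent with Leap Motion hand grabs.
; While open, right-hand OK grabs mark suspect and left-hand NotOk grabs mark innocent, recording the decision and closing the panel.
; Innocent verdicts shrink the panel and lower the roof by timeline, loading the arrested ending at bottom.
; A 30-second Tick delay ends the round, spawning police cars toward suspects.
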(event `self.ReceiveTick`
  (params (DeltaSeconds :type "Float (single-precision)"))
  (bind _roof (`self.Roof`))
  (`|ExecutionSequence`
    (:`then_0`
      (bind _aspano_game_mode (cast `/Game/Blueprints/PanoGameMode` (`GameplayStatics.GetGameMode`)))
      (bind _currentgamestate (`/Game/Blueprints/PanoGameMode.CurrentGameState` _aspano_game_mode))
      (if (`|EnumEquality` _currentgamestate "NewEnumerator2")
        (`|ExecutionSequence`
          (:`then_0`
            (bind _timer (`self.UpdateTimer` DeltaSeconds)))
          (:`then_1`
            (bind _isinnocent (`self.DecidedAsInnocent`)))
          (:`then_2`
            (bind _issuspect (`self.DecidedAsSuspect`)))
          (:`then_3`
            (if _issuspect
              (`self.SetDecision` true "NewEnumerator2" _aspano_game_mode)
              (`self.ClosePanel` _aspano_game_mode :!label _label)
              (elif _isinnocent
                (`self.SetDecision` false "NewEnumerator3" _aspano_game_mode)
                (`self.RoofPannel`)
                (goto _label))))
          (:`then_4`
            ;[1 1 1] Roof animation + Load arrested ending
            (if (`self.GoDown`)
              (bind (_direction _driver) (`Timeline|Timeline_0` :!via `PlayFromStart`)
                (:`Update`
                  (`self.K2_SetActorLocation` _roof (`KismetMathLibrary.MakeVector` 0.0 0.0 (`KismetMathLibrary.Lerp` (`self.RoofLastPos`) (`self.RoofNextPos`) _driver)) false false)
                  (set `self.GoDown` false))
                (:`Finished`
                  (if (<= (.z (`self.K2_GetActorLocation` _roof)) -860.0)
                    (`GameplayStatics.OpenLevel` "PanoEndArrested")))))))))
    (:`then_1`
      (if (`|EnumInequality` _currentgamestate "NewEnumerator4")
        (`KismetSystemLibrary.Delay` 30.0)
        (`KismetSystemLibrary.PrintString` "Ending")
        (set `/Game/Blueprints/PanoGameMode.CurrentGameState` "NewEnumerator4" _aspano_game_mode)
        (`self.SendPolice` _aspano_game_mode)))))

(fn `ClosePanel`
  (params (PanoGameState :type "/Game/Blueprints/PanoGameMode Object Reference"))
  (`SceneComponent.SetVisibility` (`self.Pannel`) false true)
  ;[1 1 1] Set PanoGameMode
  (set `/Game/Blueprints/PanoGameMode.CurrentGameState` "NewEnumerator1" PanoGameState))

(fn `DecidedAsInnocent`
  (returns (IsInnocent :type Boolean))
  (bind _leaphands (`self.LeapHands`))
  (bind _lefthandmesh (`/LeapMotion/Blueprints/Rigging/FloatingHands/LeapRiggedEchoHandsActor.LeftHandMesh` _leaphands))
  (return (and (`SceneComponent.bVisible` _lefthandmesh) (== (`PrimitiveComponent.GetMaterial` _lefthandmesh 0) "/Game/Materials/Hands/M_HandNotOk.M_HandNotOk") (`/Game/Blueprints/BP_LeapHands.bLeftHandGrabbing` _leaphands))))

(fn `DecidedAsSuspect`
  (returns (IsSuspect :type Boolean))
  (bind _leaphands (`self.LeapHands`))
  (bind _righthandmesh (`/LeapMotion/Blueprints/Rigging/FloatingHands/LeapRiggedEchoHandsActor.RightHandMesh` _leaphands))
  (return (and (`SceneComponent.bVisible` _righthandmesh) (== (`PrimitiveComponent.GetMaterial` _righthandmesh 0) "/Game/Materials/Hands/M_HandOk.M_HandOk") (`/Game/Blueprints/BP_LeapHands.bRightHandGrabbing` _leaphands))))

(fn `OpenPanel`
  ;[1 1 1] -> Called by LeapHands
  (`SceneComponent.SetVisibility` (`self.Pannel`) true true)
  ;;[1 1 1] Set PanoGameMode
  (bind _aspano_game_mode (cast `/Game/Blueprints/PanoGameMode` (`GameplayStatics.GetGameMode`)))
  (set `/Game/Blueprints/PanoGameMode.CurrentGameState` "NewEnumerator2" _aspano_game_mode))

(fn `RoofPannel`
  (returns (GoToArrestedEnding :type Boolean))
  (bind _pannel (`self.Pannel`))
  (bind _roof (`self.Roof`))
  (bind _z (.z (`SceneComponent.K2_GetComponentLocation` (`/Game/Blueprints/BP_RoomRoof.DefaultSceneRoot` _roof))))
  (bind _returnvalue (<= (.z (`SceneComponent.K2_GetComponentLocation` (`/Game/Blueprints/BP_RoomRoof.DefaultSceneRoot` _roof))) -860.0))
  (if (not _returnvalue)
    (set `self.RoofLastPos` _z)
    (set `self.RoofNextPos` (- _z 174.0))
    (set `self.GoDown` true)
    (`SceneComponent.SetWorldScale3D` _pannel (- (`SceneComponent.RelativeScale3D` _pannel) 0.46)))
  (return _returnvalue))

(fn `SendPolice`
  (params (PanoGameState :type "/Game/Blueprints/PanoGameMode Object Reference"))
  (for _array_element (`/Game/Blueprints/PanoGameMode.Decisions` PanoGameState)
    (bind (_profile _suspect) (break `/Game/Blueprints/St_ProfileDecision` _array_element))
    (if _suspect
      (`KismetArrayLibrary.Array_Add` (`self.SuspectPositions`) _profile)))
  (for _array_element_2 (`self.SuspectPositions`)
    (bind _returnvalue (`|SpawnActorFromClass` "/Game/Blueprints/BP_PoliceCarActor.BP_PoliceCarActor_C" (`KismetMathLibrary.MakeTransform` (0.0 0.0 0.0)) "Undefined" "OverrideRootScale"))
    (`SceneComponent.K2_AttachTo` (`/Game/Blueprints/BP_PoliceCarActor.BP_Root` _returnvalue) (`/Game/Blueprints/BP_CityMapActor.CIty_Ground` (`self.CityMapActor`)) "None" "KeepRelativeOffset" true)
    (set `/Game/Blueprints/BP_PoliceCarActor.TargetPosition` _array_element_2 _returnvalue)
    (set `/Game/Blueprints/BP_PoliceCarActor.Speed` (`self.PoliceSpeed`) _returnvalue)))

(fn `SetAsInnocent`)

(fn `SetDecision`
  (params (`IsSuspect?` :type Boolean) (`Warning State` :type "/Game/Blueprints/E_WarningStates Enum") (PanoGameState :type "/Game/Blueprints/PanoGameMode Object Reference"))
  (bind _alertbubble (`self.AlertBubble`))
  (`/Game/Blueprints/PanoGameMode.AddDecision` PanoGameState (make `/Game/Blueprints/St_ProfileDecision` _alertbubble `IsSuspect?`))
  (set `/Game/Blueprints/BP_AlertActor.CurrentWarningState` `Warning State` _alertbubble))

(fn `UpdateTimer`
  (params (DeltaTime :type "Float (double-precision)"))
  (returns (Timer :type "Float (double-precision)"))
  (bind _output_get (set `self.PanelTimer` (- (`self.PanelTimer`) DeltaTime)))
  (return _output_get))

(fn `UserConstructionScript`)