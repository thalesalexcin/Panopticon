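; Police car actor that drives toward a target's AlertMesh while playing police audio through Wwise.
; BeginPlay posts the police play event.
; Each Tick compares the root and AlertMesh relative locations and, beyond MinimalDistance, applies an unswept local-space offset along that direction scaled by Speed and delta time.
; Once within range it stops moving and a DoOnce posts the audio stop event.
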(event `self.ReceiveBeginPlay`
  (`AkGameplayStatics.PostEvent` "/Game/WwiseAudio/EV_ThisIsThePolicePlay.EV_ThisIsThePolicePlay" self true))

(event `self.ReceiveTick`
  (params (DeltaSeconds :type "Float (single-precision)"))
  (bind _returnvalue (`KismetMathLibrary.TransformLocation` (`SceneComponent.GetRelativeTransform` (`self.BP_Root`))))
  (bind _returnvalue_2 (`KismetMathLibrary.TransformLocation` (`SceneComponent.GetRelativeTransform` (`/Game/Blueprints/BP_AlertActor.AlertMesh` (`self.TargetPosition`)))))
  (if (> (`KismetMathLibrary.VSize` (- _returnvalue _returnvalue_2)) (`self.MinimalDistance`))
    (`self.K2_AddActorLocalOffset` (* (* (`KismetMathLibrary.GetDirectionVector` _returnvalue _returnvalue_2) DeltaSeconds) (`self.Speed`)))
    (else
      (`/Engine/EditorBlueprintResources/StandardMacros.DoOnce` false
        (:`Completed`
          (`AkGameplayStatics.PostEvent` "/Game/WwiseAudio/EV_ThisIsThePoliceStop.EV_ThisIsThePoliceStop" self true))))))

(fn `UserConstructionScript`)