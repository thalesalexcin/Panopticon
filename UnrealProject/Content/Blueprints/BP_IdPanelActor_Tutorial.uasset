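; Tutorial ID panel where the player practises judging someone innocent or suspect with Leap Motion hand gestures.
; During one tutorial state, holding a left-hand (innocent) or right-hand (suspect) grab with the matching material fills a timer that drains on release.
; The timers drive hand material parameters and Wwise loading audio.
; Either completed decision advances the tutorial, flags its trigger and destroys the alert and panel.
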(event `self.ReceiveTick`
  (params (DeltaSeconds :type "Float (single-precision)"))
  (bind _returnvalue (/ (`self.TimerSetDecision_L`) (`self.TimeToSetDecision`)))
  (bind _returnvalue_2 (/ (`self.TimerSetDecision_R`) (`self.TimeToSetDecision`)))
  (if (`self.HasDecided`)
    (`self.K2_DestroyActor` self)
    (elif (`|EnumEquality` (`/Game/Blueprints/BP_Tutorial.CurrentTutorialState` (`self.TutorialActor`)) "NewEnumerator5")
      (`|ExecutionSequence`
        (:`then_0`
          (`/Engine/EditorBlueprintResources/StandardMacros.DoOnce` false :!label _label
            (:`Completed`
              (`AkGameplayStatics.PostEvent` "/Game/WwiseAudio/EV_LoadingHand.EV_LoadingHand" self true)
              (goto _label_3 :!via `Reset`))))
        (:`then_1`
          (bind _isinnocent (`self.DecidedAsInnocent` DeltaSeconds))
          (if _isinnocent
            (`self.K2_DestroyActor` (`self.AlertTutorial`) :!label _label_2)
            (set `/Game/Blueprints/BP_TriggersSelection_Tutorial.HasDecided` true (`self.TriggerTutorial`))
            (set `/Game/Blueprints/BP_Tutorial.CurrentTutorialState` "NewEnumerator7" (`self.TutorialActor`))
            (`self.K2_DestroyActor`)))
        (:`then_2`
          (bind _issuspect (`self.DecidedAsSuspect` DeltaSeconds))
          (if _issuspect
            (goto _label_2)))
        (:`then_3`
          (`KismetMaterialLibrary.SetScalarParameterValue` "/Game/Materials/Hands/HandsMaterial.HandsMaterial" "RightHandTimer" _returnvalue_2)
          (`KismetMaterialLibrary.SetScalarParameterValue` "/Game/Materials/Hands/HandsMaterial.HandsMaterial" "LeftHandTimer" _returnvalue)
          (`AkGameplayStatics.SetRTPCValue` "LoadingHand" (`KismetMathLibrary.FMax` (* _returnvalue_2 100.0) (* _returnvalue 100.0)) 0 self)))
      (else
        (`/Engine/EditorBlueprintResources/StandardMacros.DoOnce` false :!label _label_3
          (:`Completed`
            (`AkGameplayStatics.PostEvent` "/Game/WwiseAudio/EV_LoadingHandStop.EV_LoadingHandStop" self true)
            (`|ExecutionSequence`
              (:`then_0`
                (set `self.TimerSetDecision_R` 0.0)
                (set `self.TimerSetDecision_L` 0.0))
              (:`then_1`
                (goto _label :!via `Reset`)))))))))

(fn `DecidedAsInnocent`
  (params (DeltaTime :type "Float (double-precision)"))
  (returns (IsInnocent :type Boolean))
  (bind _timersetdecision_l (`self.TimerSetDecision_L`))
  (bind _leaphands (`self.LeapHands`))
  (bind _lefthandmesh (`/LeapMotion/Blueprints/Rigging/FloatingHands/LeapRiggedEchoHandsActor.LeftHandMesh` _leaphands))
  (if (and (`SceneComponent.bVisible` _lefthandmesh) (== (`PrimitiveComponent.GetMaterial` _lefthandmesh 0) "/Game/Materials/Hands/M_HandNotOk.M_HandNotOk") (`/Game/Blueprints/BP_LeapHands.bLeftHandGrabbing` _leaphands))
    (set `self.TimerSetDecision_L` (+ _timersetdecision_l DeltaTime))
    (elif (>= _timersetdecision_l 0.0)
      (set `self.TimerSetDecision_L` (- _timersetdecision_l DeltaTime))
      (else
        (set `self.TimerSetDecision_L` 0.0))))
  (return (>= (`self.TimerSetDecision_L`) (`self.TimeToSetDecision`))))

(fn `DecidedAsSuspect`
  (params (DeltaTime :type "Float (double-precision)"))
  (returns (IsSuspect :type Boolean))
  (bind _timersetdecision_r (`self.TimerSetDecision_R`))
  (bind _leaphands (`self.LeapHands`))
  (bind _righthandmesh (`/LeapMotion/Blueprints/Rigging/FloatingHands/LeapRiggedEchoHandsActor.RightHandMesh` _leaphands))
  (if (and (`SceneComponent.bVisible` _righthandmesh) (== (`PrimitiveComponent.GetMaterial` _righthandmesh 0) "/Game/Materials/Hands/M_HandOk.M_HandOk") (`/Game/Blueprints/BP_LeapHands.bRightHandGrabbing` _leaphands))
    (set `self.TimerSetDecision_R` (+ _timersetdecision_r DeltaTime))
    (elif (>= _timersetdecision_r 0.0)
      (set `self.TimerSetDecision_R` (- _timersetdecision_r DeltaTime))
      (else
        (set `self.TimerSetDecision_R` 0.0))))
  (return (>= (`self.TimerSetDecision_R`) (`self.TimeToSetDecision`))))

(fn `OpenPanel`
  ;[1 1 1] -> Called by LeapHands
  (`SceneComponent.SetVisibility` (`self.Pannel`) true true))

(fn `SetAsInnocent`)

(fn `UserConstructionScript`)