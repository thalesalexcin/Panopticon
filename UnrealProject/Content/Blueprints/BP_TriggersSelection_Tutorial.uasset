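; BP_TriggersSelection_Tutorial gives hand feedback for a two-sided tutorial choice, with a Left "not OK" trigger and a Right "OK" trigger.
; Each Tick checks whether each hand mesh overlaps its same-side trigger, swapping between highlight and default materials.
; SetCustomMaterial changes the material and posts the Wwise confirm in/out event only when the material differs.
; Once HasDecided is true, it restores both default hand materials and destroys itself.
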(event `self.ReceiveTick`
  (params (DeltaSeconds :type "Float (single-precision)"))
  (bind _hands (`self.Hands`))
  (bind _lefthandmesh (`/LeapMotion/Blueprints/Rigging/FloatingHands/LeapRiggedEchoHandsActor.LeftHandMesh` _hands))
  (bind _righthandmesh (`/LeapMotion/Blueprints/Rigging/FloatingHands/LeapRiggedEchoHandsActor.RightHandMesh` _hands))
  (if (`self.HasDecided`)
    ;[1 1 1] Default Material
    (`|ExecutionSequence`
      (:`then_0`
        (`self.SetCustomMaterial` (`/LeapMotion/Blueprints/Rigging/FloatingHands/LeapRiggedEchoHandsActor.LeftHandMesh` _hands) "/Game/Materials/Hands/M_Hands_L.M_Hands_L"))
      (:`then_1`
        (`self.SetCustomMaterial` (`/LeapMotion/Blueprints/Rigging/FloatingHands/LeapRiggedEchoHandsActor.RightHandMesh` _hands) "/Game/Materials/Hands/M_Hands_R.M_Hands_R")
        (`self.K2_DestroyActor`)))
    (else
      (`|ExecutionSequence`
        (:`then_0`
          ;[1 1 1] LeftHand Material
          (if (`PrimitiveComponent.IsOverlappingComponent` (`self.Left`) _lefthandmesh)
            (`self.SetCustomMaterial` _lefthandmesh "/Game/Materials/Hands/M_HandNotOk.M_HandNotOk" "/Game/WwiseAudio/EV_ConfirmIn.EV_ConfirmIn")
            (else
              (`self.SetCustomMaterial` _lefthandmesh "/Game/Materials/Hands/M_Hands_L.M_Hands_L" "/Game/WwiseAudio/EV_ConfirmOut.EV_ConfirmOut"))))
        (:`then_1`
          ;[1 1 1] RightHand Material
          (if (`PrimitiveComponent.IsOverlappingComponent` (`self.Right`) _righthandmesh)
            (`self.SetCustomMaterial` _righthandmesh "/Game/Materials/Hands/M_HandOk.M_HandOk" "/Game/WwiseAudio/EV_ConfirmIn.EV_ConfirmIn")
            (else
              (`self.SetCustomMaterial` _righthandmesh "/Game/Materials/Hands/M_Hands_R.M_Hands_R" "/Game/WwiseAudio/EV_ConfirmOut.EV_ConfirmOut"))))))))

(fn `SetCustomMaterial`
  (params (HandMesh :type "PrimitiveComponent Object Reference") (MatToSet :type "Material Object Reference") (AkEvent :type "AkAudioEvent Object Reference"))
  (if (!= (`PrimitiveComponent.GetMaterial` HandMesh 0) MatToSet)
    (`PrimitiveComponent.SetMaterial` HandMesh 0 MatToSet)
    (`AkGameplayStatics.PostEvent` AkEvent self true))
  (return))

(fn `UserConstructionScript`)