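; Floating warning bubble, drawn as a Paper2D flipbook, that billboards to the player camera and plays Wwise audio.
; While PanoGameMode is in either of two game states, Tick advances a timer and runs a state machine.
; Grow raises and scales the bubble into Idle, which floats and can turn translucent when deciding; Eye morphs it, and Pop destroys it.
; RTPCs drive growth sound and scale-corrected distance attenuation.
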(event `self.ReceiveBeginPlay`
  (bind _paperflipbook (`self.PaperFlipbook`))
  (`PaperFlipbookComponent.Stop` _paperflipbook)
  (`PaperFlipbookComponent.SetLooping` _paperflipbook false))

(event `self.ReceiveTick`
  (params (DeltaSeconds :type "Float (single-precision)"))
  (`|ExecutionSequence`
    (:`then_0`
      (`self.LookAt`))
    (:`then_1`
      (bind _aspano_game_mode (cast `/Game/Blueprints/PanoGameMode` (`GameplayStatics.GetGameMode`)))
      (bind _currentgamestate (`/Game/Blueprints/PanoGameMode.CurrentGameState` _aspano_game_mode))
      (if (or (`|EnumEquality` _currentgamestate "NewEnumerator1") (`|EnumEquality` _currentgamestate "NewEnumerator2"))
        (`|ExecutionSequence`
          (:`then_0`
            (`self.SetTimer` DeltaSeconds))
          (:`then_1`
            (switch `/Game/Blueprints/E_WarningStates` (`self.CurrentWarningState`)
              (:`NewEnumerator0`
                (`self.GrowState` DeltaSeconds "/Game/WwiseAudio/EV_PopWarningPlay.EV_PopWarningPlay"))
              (:`NewEnumerator1`
                (`self.IdleState` DeltaSeconds :!label _label))
              (:`NewEnumerator4`
                (goto _label))
              (:`NewEnumerator2`
                (`self.EyeState` "/Game/WwiseAudio/EV_PopWarningStop.EV_PopWarningStop" "/Game/WwiseAudio/EV_WarningEye.EV_WarningEye"))
              (:`NewEnumerator3`
                (`self.PopState` "/Game/WwiseAudio/EV_PopWarningStop.EV_PopWarningStop" "/Game/WwiseAudio/EV_PopWW.EV_PopWW"))))
          (:`then_2`
            ;[1 1 1] WIP Distance to player (RTPC Atenuation)
            (`AkGameplayStatics.SetRTPCValue` "WarningAttenuation" (* (/ 1.0 (.x (`SceneComponent.RelativeScale3D` (`SceneComponent.GetAttachParent` (`SceneComponent.GetAttachParent` (`SceneComponent.GetAttachParent` (`self.AlertMesh`))))))) (`self.GetDistanceTo` (`GameplayStatics.GetPlayerController` 0))) 0 self)))))
    (:`then_2`)))

(fn `EyeState`
  (params (AkEventToStop :type "AkAudioEvent Object Reference") (AkEventToPlay :type "AkAudioEvent Object Reference") (DeltaTime :type "Float (double-precision)"))
  (bind _paperflipbook (`self.PaperFlipbook`))
  (`|ExecutionSequence`
    (:`then_0`
      (if (`self.DoEye`)
        (`PaperFlipbookComponent.SetFlipbook` _paperflipbook "/Game/Textures/Pictograms/Flipbooks/Warning/FB_WarningToEye.FB_WarningToEye")
        (`PaperFlipbookComponent.SetLooping` _paperflipbook false)
        (`PrimitiveComponent.SetMaterial` _paperflipbook 0 "/Paper2D/MaskedUnlitSpriteMaterial.MaskedUnlitSpriteMaterial")
        (`AkGameplayStatics.PostEvent` AkEventToStop self true)
        (`AkGameplayStatics.PostEvent` AkEventToPlay self true)
        (set `self.DoEye` false)))
    (:`then_1`
      (`PaperFlipbookComponent.Play` _paperflipbook)
      (`self.FloatingEffect` DeltaTime)
      (return))))

(fn `FloatingEffect`
  (params (DeltaTime :type "Float (double-precision)"))
  (bind _alertmesh (`self.AlertMesh`))
  (bind _returnvalue (* (`self.Timer`) (`self.FloatingSpeed_Z`)))
  (bind _returnvalue_2 (* (`self.Timer`) (`self.FloatingSpeed_Y`)))
  (`SceneComponent.K2_AddLocalOffset` _alertmesh (`KismetMathLibrary.InverseTransformDirection` (`SceneComponent.GetRelativeTransform` _alertmesh) (`KismetMathLibrary.MakeVector` 0.0 (* (- (`KismetMathLibrary.Sin` (+ DeltaTime _returnvalue_2)) (`KismetMathLibrary.Sin` _returnvalue_2)) (`self.FloatingAmplitude_Y`)) (* (- (`KismetMathLibrary.Sin` (+ DeltaTime _returnvalue)) (`KismetMathLibrary.Sin` _returnvalue)) (`self.FloatingAmplitude_Z`)))) false false)
  (return))

(fn `GrowState`
  (params (DeltaTime :type "Float (double-precision)") (AkEvent :type "AkAudioEvent Object Reference"))
  (bind _alertmesh (`self.AlertMesh`))
  (bind _alertmesh_2 (`self.AlertMesh`))
  (bind _paperflipbook (`self.PaperFlipbook`))
  (bind _paperflipbook_2 (`self.PaperFlipbook`))
  (bind _returnvalue (* (`self.Timer`) 10.0))
  (bind _relativescale3d (`SceneComponent.RelativeScale3D` _alertmesh_2))
  (`|ExecutionSequence`
    (:`then_0`
      ;[1 1 1] Ak Grow
      (if (<= _returnvalue 75.0)
        (`AkGameplayStatics.SetRTPCValue` "Grow" _returnvalue 0 self)
        (if (`self.DoGrow`)
          (`AkGameplayStatics.PostEvent` AkEvent self true)
          (set `self.DoGrow` false))
        (else
          (`AkGameplayStatics.SetRTPCValue` "Grow" 75.0 0 self))))
    (:`then_1`
      ;[1 1 1] Up
      (`SceneComponent.K2_AddLocalOffset` _alertmesh (`KismetMathLibrary.InverseTransformDirection` (`SceneComponent.GetRelativeTransform` _alertmesh) (* (0.0 0.0 300.0) DeltaTime)) false false))
    (:`then_2`
      ;[1 1 1] Scale
      (`SceneComponent.SetRelativeScale3D` _alertmesh_2 (+ _relativescale3d (* (* (+ _relativescale3d (1.0 1.0 1.0)) 0.08) DeltaTime))))
    (:`then_3`
      ;[1 1 1] TimeBeforMorph
      (if (>= (`self.Timer`) (`self.CapsuleToPictoTime`))
        (`PaperFlipbookComponent.SetPlayRate` _paperflipbook (`self.BubblePlayRate`))
        (`PaperFlipbookComponent.Play` _paperflipbook)))
    (:`then_4`
      ;[1 1 1] Destroy - Stop Up & Scale - Go To Idle
      (if (>= (`PaperFlipbookComponent.GetPlaybackPositionInFrames` _paperflipbook_2) (- (`PaperFlipbookComponent.GetFlipbookLengthInFrames` _paperflipbook_2) 1))
        (set `self.CurrentWarningState` "NewEnumerator1")
        (return)))))

(fn `IdleState`
  (params (DeltaTime :type "Float (double-precision)"))
  (bind _paperflipbook (`self.PaperFlipbook`))
  ;[1 1 1] Mvt
  (`self.FloatingEffect` DeltaTime)
  (`|ExecutionSequence`
    (:`then_0`
      (if (`self.DoIdle`)
        (`PaperFlipbookComponent.SetFlipbook` _paperflipbook "/Game/Textures/Pictograms/Flipbooks/Warning/FB_Warning_Idle.FB_Warning_Idle")
        (`PaperFlipbookComponent.SetLooping` _paperflipbook true)
        (set `self.DoIdle` false)
        (else
          (`PaperFlipbookComponent.Play` _paperflipbook :!label _label))))
    (:`then_1`
      (goto _label))
    (:`then_2`
      ;[1 1 1] Set Invisible when deciding
      (bind _aspano_game_mode (cast `/Game/Blueprints/PanoGameMode` (`GameplayStatics.GetGameMode`))
        (:`then`
          (if (and (`self.DoTransparency`) (`|EnumEquality` (`/Game/Blueprints/PanoGameMode.CurrentGameState` _aspano_game_mode) "NewEnumerator2") (`|EnumEquality` (`self.CurrentWarningState`) "NewEnumerator4"))
            (`PrimitiveComponent.SetMaterial` _paperflipbook 0 "/Paper2D/TranslucentUnlitSpriteMaterial.TranslucentUnlitSpriteMaterial")
            (set `self.DoTransparency` false)))
        (:`CastFailed`
          _))
      (return))))

(fn `LookAt`
  (`self.SetActorRotation` (`KismetMathLibrary.MakeRotFromX` (- (`SceneComponent.K2_GetComponentLocation` (`self.PaperFlipbook`)) (`self.K2_GetActorLocation` (`GameplayStatics.GetPlayerCameraManager` 0)))))
  (return))

(fn `PopState`
  (params (AkEventToStop :type "AkAudioEvent Object Reference") (AkEventToPlay :type "AkAudioEvent Object Reference"))
  (bind _paperflipbook (`self.PaperFlipbook`))
  (bind _paperflipbook_2 (`self.PaperFlipbook`))
  (`|ExecutionSequence`
    (:`then_0`
      (if (`self.DoPop`)
        (`PaperFlipbookComponent.SetFlipbook` _paperflipbook "/Game/Textures/Pictograms/Flipbooks/Warning/FB_Warning_Pop.FB_Warning_Pop")
        (`PaperFlipbookComponent.SetLooping` _paperflipbook false)
        (`AkGameplayStatics.PostEvent` AkEventToStop self true)
        (`AkGameplayStatics.PostEvent` AkEventToPlay self true)
        (set `self.DoPop` false)))
    (:`then_1`
      (`PaperFlipbookComponent.Play` _paperflipbook))
    (:`then_2`
      ;[1 1 1] Destroy
      (if (>= (`PaperFlipbookComponent.GetPlaybackPositionInFrames` _paperflipbook_2) (- (`PaperFlipbookComponent.GetFlipbookLengthInFrames` _paperflipbook_2) 1))
        (`self.K2_DestroyActor`)
        (else
          (return))))))

(fn `SetTimer`
  (params (DeltaSeconds :type "Float (double-precision)"))
  (set `self.Timer` (+ (`self.Timer`) DeltaSeconds))
  (return))

(fn `UserConstructionScript`)