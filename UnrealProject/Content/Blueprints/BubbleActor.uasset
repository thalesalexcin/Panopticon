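; BubbleActor is an actor that acts as a short-lived rising bubble.
; Each Tick moves the Bubble component upward along its local Z at a steady, frame-rate-independent speed and steadily grows its relative scale in proportion to its current size.
; BeginPlay starts a timer that calls DestroyBubble after a few seconds to remove the actor.
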(event `self.ReceiveBeginPlay`
  (`KismetSystemLibrary.K2_SetTimer` null "DestroyBubble" 4.0))

(event `self.ReceiveTick`
  (params (DeltaSeconds :type "Float (single-precision)"))
  (bind _bubble (`self.Bubble`))
  (bind _relativescale3d (`SceneComponent.RelativeScale3D` _bubble))
  (`|ExecutionSequence`
    (:`then_0`
      (`SceneComponent.K2_AddLocalOffset` _bubble (* (0.0 0.0 300.0) DeltaSeconds) false false))
    (:`then_1`
      (`SceneComponent.SetRelativeScale3D` _bubble (+ _relativescale3d (* (* (+ _relativescale3d (1.0 1.0 1.0)) 0.08) DeltaSeconds))))))

(fn `DestroyBubble`
  (`self.K2_DestroyActor`)
  (return))

(fn `UserConstructionScript`)