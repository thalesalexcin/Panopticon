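; PanoGameMode is a game mode that holds the current game state and the list of player decisions.
; Construction sets the state to Starting, and CanMoveMap allows map movement only while Poping or Tutorialing.
; AddDecision only appends to Decisions; its unwired leftover logic would arrest the player after too many consecutive innocent profiles, with a note pointing to Id_PanelActor.
; The event graph's state switch and delayed change to Poping are also disconnected.
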(fn `AddDecision`
  (params (Decision :type "/Game/Blueprints/St_ProfileDecision Structure"))
  (`KismetArrayLibrary.Array_Add` (`self.Decisions`) Decision))

(fn `CanMoveMap`
  (returns (CanMoveMap :type Boolean))
  (bind _currentgamestate (`self.CurrentGameState`))
  (return (or (`|EnumEquality` _currentgamestate "NewEnumerator1") (`|EnumEquality` _currentgamestate "NewEnumerator5") false)))

(fn `UserConstructionScript`
  (set `self.CurrentGameState` "NewEnumerator0"))