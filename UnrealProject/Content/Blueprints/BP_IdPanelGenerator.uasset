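; Actor that spawns a timed series of profile alert actors onto the city map from a configured profile list.
; On BeginPlay it walks the list, using each entry's delay from the previous one to set a timer by function name.
; Each timer spawns a BP_AlertActor at the entry's world position, attaches it to the map ground, assigns its sprite, then schedules the next.
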(event `self.ReceiveBeginPlay`
  (set `self.ProfileIndex` 0)
  (`self.GenerateAlert`))

(fn `GenerateAlert`
  (bind _profilestogenerater (`self.ProfilesToGenerater`))
  (bind _profileindex (`self.ProfileIndex`))
  (if (< _profileindex (`KismetArrayLibrary.Array_Length` _profilestogenerater))
    (`KismetSystemLibrary.K2_SetTimer` null "SetGenerateAlertTimer" (`.DelayFromLastProfile_6_F1B5F99544206197430A1CBAB00053EF` (break `/Game/Blueprints/IdPanelInfo` (`KismetArrayLibrary.Array_Get` _profilestogenerater _profileindex)))))
  (return))

(fn `SetGenerateAlertTimer`
  (bind (_worldposition _profile) (break `/Game/Blueprints/IdPanelInfo` (`KismetArrayLibrary.Array_Get` (`self.ProfilesToGenerater`) (`self.ProfileIndex`))))
  (`|ExecutionSequence`
    (:`then_0`
      (bind _returnvalue (`|SpawnActorFromClass` "/Game/Blueprints/BP_AlertActor.BP_AlertActor_C" (`KismetMathLibrary.Conv_VectorToTransform` _worldposition) "AlwaysSpawn" "OverrideRootScale"))
      (`self.K2_AttachRootComponentTo` _returnvalue (`/Game/Blueprints/BP_CityMapActor.CIty_Ground` (`self.CityMap`)) "None" "KeepRelativeOffset" true)
      (set `/Game/Blueprints/BP_AlertActor.ProfileSprite` _profile _returnvalue))
    (:`then_1`
      (`/Engine/EditorBlueprintResources/StandardMacros.IncrementInt` (`self.ProfileIndex`)
        (:`  `
          (`self.GenerateAlert`)
          (return))))))

(fn `UserConstructionScript`)