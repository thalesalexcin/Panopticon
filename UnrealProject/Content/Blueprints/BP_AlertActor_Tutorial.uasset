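; BP_AlertActor_Tutorial is a tutorial warning alert, shown as a looping flipbook, that the player triggers with Leap hands.
; While idle, Tick checks whether either hand mesh overlaps AlertTrigger.
; On touch it spawns selection triggers near the camera and an ID panel, wires their references, and advances the tutorial state.
; It then enters IdleDeciding, swapping to a translucent material once; LookAt and SetTimer helpers are never called here.
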(event `self.ReceiveBeginPlay`
  (set `self.CurrentWarningState` "NewEnumerator1")
  (`PaperFlipbookComponent.SetLooping` (`self.PaperFlipbook`) true))

(event `self.ReceiveTick`
  (params (DeltaSeconds :type "Float (single-precision)"))
  (`|ExecutionSequence`
    (:`then_0`
      (`PaperFlipbookComponent.Play` (`self.PaperFlipbook`)))
    (:`then_1`
      (switch `/Game/Blueprints/E_WarningStates` (`self.CurrentWarningState`)
        (:`NewEnumerator1`
          (`self.IdleState`))
        (:`NewEnumerator4`
          (`/Engine/EditorBlueprintResources/StandardMacros.DoOnce` false
            (:`Completed`
              (`PrimitiveComponent.SetMaterial` (`self.PaperFlipbook`) 0 "/Paper2D/TranslucentUnlitSpriteMaterial.TranslucentUnlitSpriteMaterial"))))))))

(fn `IdleState`
  (bind _hands (`self.Hands`))
  (bind _hands_2 (`self.Hands`))
  (bind _alerttrigger (`self.AlertTrigger`))
  (`PaperFlipbookComponent.Play` (`self.PaperFlipbook`))
  (if (or (`PrimitiveComponent.IsOverlappingComponent` _alerttrigger (`/LeapMotion/Blueprints/Rigging/FloatingHands/LeapRiggedEchoHandsActor.LeftHandMesh` _hands_2)) (`PrimitiveComponent.IsOverlappingComponent` _alerttrigger (`/LeapMotion/Blueprints/Rigging/FloatingHands/LeapRiggedEchoHandsActor.RightHandMesh` _hands_2)))
    (bind _returnvalue (`|SpawnActorFromClass` "/Game/Blueprints/BP_TriggersSelection_Tutorial.BP_TriggersSelection_Tutorial_C" (`KismetMathLibrary.MakeTransform` (`KismetMathLibrary.MakeVector` (+ (.x (`PlayerCameraManager.GetCameraLocation` (`GameplayStatics.GetPlayerCameraManager` 0))) 20.0) (.y (`PlayerCameraManager.GetCameraLocation` (`GameplayStatics.GetPlayerCameraManager` 0))) (+ (.z (`PlayerCameraManager.GetCameraLocation` (`GameplayStatics.GetPlayerCameraManager` 0))) 30.0))) "Undefined" "OverrideRootScale"))
    (set `/Game/Blueprints/BP_TriggersSelection_Tutorial.Hands` _hands _returnvalue)
    (bind _returnvalue_2 (`|SpawnActorFromClass` "/Game/Blueprints/BP_IdPanelActor_Tutorial.BP_IdPanelActor_Tutorial_C" (`KismetMathLibrary.MakeTransform` (0.0 0.0 0.0)) "Undefined" "OverrideRootScale"))
    (set `/Game/Blueprints/BP_IdPanelActor_Tutorial.LeapHands` _hands _returnvalue_2)
    (set `/Game/Blueprints/BP_IdPanelActor_Tutorial.TriggerTutorial` _returnvalue _returnvalue_2)
    (set `/Game/Blueprints/BP_IdPanelActor_Tutorial.AlertTutorial` self _returnvalue_2)
    (set `/Game/Blueprints/BP_IdPanelActor_Tutorial.TutorialActor` (`self.TutorialActor`) _returnvalue_2)
    (set `/Game/Blueprints/BP_Tutorial.CurrentTutorialState` "NewEnumerator5" (`self.TutorialActor`))
    (set `self.CurrentWarningState` "NewEnumerator4")))

(fn `LookAt`
  (`self.SetActorRotation` (`KismetMathLibrary.MakeRotFromX` (- (`SceneComponent.K2_GetComponentLocation` (`self.PaperFlipbook`)) (`self.K2_GetActorLocation` (`GameplayStatics.GetPlayerCameraManager` 0))))))

(fn `SetTimer`
  (params (DeltaTime :type "Float (double-precision)"))
  (set `self.Timer` (+ (`self.Timer`) DeltaTime)))

(fn `UserConstructionScript`)