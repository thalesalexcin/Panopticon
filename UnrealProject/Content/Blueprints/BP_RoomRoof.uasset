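; BP_RoomRoof is a room roof actor that moves toward the world origin when the game reaches a specific state.
; Each Tick it casts the game mode to PanoGameMode and, while CurrentGameState matches that state, calls PlayFromStart on a timeline.
; The timeline lerps the actor's current Z toward zero and sets X and Y to zero.
; Because the trigger is on Tick, the timeline restarts every frame while the state holds.
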(event `self.ReceiveTick`
  (params (DeltaSeconds :type "Float (single-precision)"))
  (bind _aspano_game_mode (cast `/Game/Blueprints/PanoGameMode` (`GameplayStatics.GetGameMode`)))
  (if (`|EnumEquality` (`/Game/Blueprints/PanoGameMode.CurrentGameState` _aspano_game_mode) "NewEnumerator4")
    (bind (_direction _driver) (`Timeline|Timeline_0` :!via `PlayFromStart`)
      (:`Update`
        (`self.K2_SetActorLocation` (`KismetMathLibrary.MakeVector` 0.0 0.0 (`KismetMathLibrary.Lerp` (.z (`self.K2_GetActorLocation`)) 0.0 _driver)))))))

(fn `UserConstructionScript`)