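; Leap Motion hands actor that lets the player inspect alert actors by touch and control an ID panel with swipes.
; When either hand mesh begins overlapping a BP_AlertActor, the panel shows that actor's profile sprite, unless either hand is grabbing.
; Left and right grab inputs set the grabbing flags.
; Enabled swipe gestures show the panel on a left swipe and hide it on a right swipe.
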(event `self.ReceiveBeginPlay`
  (`parent.ReceiveBeginPlay`)
  (`self.EnableInput` (`GameplayStatics.GetPlayerController` 0))
  (`LeapController.EnableGesture` (`self.LeapController`) "GESTURE_TYPE_SWIPE" true))

(event `self.ReceiveTick`
  (params (DeltaSeconds :type "Float (single-precision)")))

(event `Key|LeapRightGrab`
  (params (Key :type "Key Structure" :default "LeapLeftPinch"))
  (:`Pressed`
    (set `self.bRightHandGrabbing` true))
  (:`Released`
    (set `self.bRightHandGrabbing` false)))

(event `Key|LeapLeftGrab` :consume false
  (params (Key :type "Key Structure" :default "LeapLeftPinch"))
  (:`Pressed`
    (set `self.bLeftHandGrabbing` true))
  (:`Released`
    (set `self.bLeftHandGrabbing` false)))

(event `self.LeftHandMesh.OnComponentBeginOverlap`
  (params (OtherActor :type "Actor Object Reference") (OtherComp :type "PrimitiveComponent Object Reference") (OtherBodyIndex :type Integer) (bFromSweep :type Boolean) (SweepResult :type "HitResult Structure (by ref)"))
  (bind _idpanel (`self.IdPanel`))
  (if (and (not (`self.bRightHandGrabbing`)) (not (`self.bLeftHandGrabbing`)))
    (bind _asbp_alert_actor (cast `/Game/Blueprints/BP_AlertActor` OtherActor))
    (`PaperSpriteComponent.SetSprite` (`/Game/Blueprints/BP_IdPanelActor.PaperSprite` _idpanel) (`/Game/Blueprints/BP_AlertActor.ProfileSprite` _asbp_alert_actor))
    (`SceneComponent.SetVisibility` (`/Game/Blueprints/BP_IdPanelActor.DefaultSceneRoot1` _idpanel) true true :!label _label)))

(event `self.RightHandMesh.OnComponentBeginOverlap`
  (params (OtherActor :type "Actor Object Reference") (OtherComp :type "PrimitiveComponent Object Reference") (OtherBodyIndex :type Integer) (bFromSweep :type Boolean) (SweepResult :type "HitResult Structure (by ref)"))
  (if (and (not (`self.bRightHandGrabbing`)) (not (`self.bLeftHandGrabbing`)))
    (bind _asbp_alert_actor (cast `/Game/Blueprints/BP_AlertActor` OtherActor))
    (`PaperSpriteComponent.SetSprite` (`/Game/Blueprints/BP_IdPanelActor.PaperSprite` (`self.IdPanel`)) (`/Game/Blueprints/BP_AlertActor.ProfileSprite` _asbp_alert_actor))
    (goto _label)))

(event `LeapEventInterface.SwipeGestureDetected`
  (params (gesture :type "LeapSwipeGesture Object Reference"))
  (bind _defaultsceneroot1 (`/Game/Blueprints/BP_IdPanelActor.DefaultSceneRoot1` (`self.IdPanel`)))
  (switch `LeapBasicDirection` (`LeapSwipeGesture.BasicDirection` gesture)
    (:`DIRECTION_LEFT`
      (`SceneComponent.SetVisibility` _defaultsceneroot1 true true))
    (:`DIRECTION_RIGHT`
      (`SceneComponent.SetVisibility` _defaultsceneroot1 false true))))

(fn `UserConstructionScript`)