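; LeapHands is a Blueprint for a pair of hand meshes driven by Leap grab input, apparently for Leap Motion hand tracking.
; Left and right grab key presses and releases set a grabbing flag for each hand.
; When either hand mesh begins an overlap while that hand is not grabbing, both paths share one placeholder that prints "Hello", commented "Open ID".
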(event `Key|LeapLeftGrab`
  (params (Key :type "Key Structure" :default "LeapLeftPinch"))
  (:`Pressed`
    (set `self.bLeftHandGrabbing` true))
  (:`Released`
    (set `self.bLeftHandGrabbing` false)))

(event `Key|LeapRightGrab`
  (params (Key :type "Key Structure" :default "LeapLeftPinch"))
  (:`Pressed`
    (set `self.bRightHandGrabbing` true))
  (:`Released`
    (set `self.bRightHandGrabbing` false)))

(event `self.LeftHandMesh.OnComponentBeginOverlap`
  (params (OtherActor :type "Actor Object Reference") (OtherComp :type "PrimitiveComponent Object Reference") (OtherBodyIndex :type Integer) (bFromSweep :type Boolean) (SweepResult :type "HitResult Structure (by ref)"))
  (if (not (`self.bLeftHandGrabbing`))
    ;[1 1 1] Open ID
    (`KismetSystemLibrary.PrintString` "Hello" :!label _label)))

(event `self.RightHandMesh.OnComponentBeginOverlap`
  (params (OtherActor :type "Actor Object Reference") (OtherComp :type "PrimitiveComponent Object Reference") (OtherBodyIndex :type Integer) (bFromSweep :type Boolean) (SweepResult :type "HitResult Structure (by ref)"))
  (if (not (`self.bRightHandGrabbing`))
    (goto _label)))

(fn `UserConstructionScript`)