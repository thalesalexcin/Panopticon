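; BP_BubbleActor is a rising bubble that shows an icon for its BubbleType category and destroys itself on a five-second timer.
; Tick moves and grows the bubble, selects the matching stopped Paper2D flipbook, and rotates the actor along the camera-to-flipbook direction as a billboard.
; A Wwise grow sound starts on BeginPlay, with its Grow RTPC driven by the destroy timer's elapsed time.
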(event `self.ReceiveBeginPlay`
  (`|ExecutionSequence`
    (:`then_0`
      (bind _returnvalue (`KismetSystemLibrary.K2_SetTimer` null "DestroyBubble" 5.0)))
    (:`then_1`
      (`AkGameplayStatics.PostEvent` "/Game/WwiseAudio/EV_Grow.EV_Grow" self true))))

(event `self.ReceiveActorBeginOverlap`
  (params (OtherActor :type "Actor Object Reference")))

(event `self.ReceiveTick`
  (params (DeltaSeconds :type "Float (single-precision)"))
  (bind _paperflipbook (`self.PaperFlipbook`))
  (bind _bubble (`self.Bubble`))
  (bind _relativescale3d (`SceneComponent.RelativeScale3D` _bubble))
  (`|ExecutionSequence`
    (:`then_0`
      (`SceneComponent.K2_AddLocalOffset` _bubble (* (0.0 0.0 300.0) DeltaSeconds) false false))
    (:`then_1`
      (`SceneComponent.SetRelativeScale3D` _bubble (+ _relativescale3d (* (* (+ _relativescale3d (1.0 1.0 1.0)) 0.08) DeltaSeconds))))
    (:`then_2`
      (`AkGameplayStatics.SetRTPCValue` "Grow" (* (`KismetSystemLibrary.K2_GetTimerElapsedTimeHandle` (stale `self.ReceiveBeginPlay` _returnvalue)) 10.0) 0 self))
    (:`then_3`
      (switch `EBubbleType` (`self.bubbleType`)
        (:`Animals`
          (`PaperFlipbookComponent.SetFlipbook` _paperflipbook "/Game/Textures/Pictograms/FB_Animals.FB_Animals"))
        (:`Food`
          (`PaperFlipbookComponent.SetFlipbook` _paperflipbook "/Game/Textures/Pictograms/FB_Food.FB_Food"))
        (:`Games`
          (`PaperFlipbookComponent.SetFlipbook` _paperflipbook "/Game/Textures/Pictograms/FB_Games.FB_Games"))
        (:`Meteorology`
          (`PaperFlipbookComponent.SetFlipbook` _paperflipbook "/Game/Textures/Pictograms/FB_Meteorology.FB_Meteorology"))
        (:`Money`
          (`PaperFlipbookComponent.SetFlipbook` _paperflipbook "/Game/Textures/Pictograms/FB_Money.FB_Money"))
        (:`Puzzle`
          (`PaperFlipbookComponent.SetFlipbook` _paperflipbook "/Game/Textures/Pictograms/FB_Puzzle.FB_Puzzle"))
        (:`Recycle`
          (`PaperFlipbookComponent.SetFlipbook` _paperflipbook "/Game/Textures/Pictograms/FB_Recycle.FB_Recycle"))
        (:`Studys`
          (`PaperFlipbookComponent.SetFlipbook` _paperflipbook "/Game/Textures/Pictograms/FB_Studys.FB_Studys")))
      (`PaperFlipbookComponent.Stop` (`self.PaperFlipbook`)))
    (:`then_4`
      (`self.SetActorRotation` (`KismetMathLibrary.MakeRotFromX` (- (`SceneComponent.K2_GetComponentLocation` (`self.PaperFlipbook`)) (`self.K2_GetActorLocation` (`GameplayStatics.GetPlayerCameraManager` 0))))))))

(fn `DestroyBubble`
  (`self.K2_DestroyActor`)
  (return))

(fn `UserConstructionScript`)