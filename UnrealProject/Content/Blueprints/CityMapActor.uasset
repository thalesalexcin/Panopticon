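; City map actor that passes Leap Motion hand gestures and keyboard zoom input to a CityMap.
; Each Tick caches both middle-finger socket positions from the Hands meshes, then feeds the right-hand position to CityMap's grab position while grabbing, or zero otherwise.
; Add and Subtract keys hold CityMap's zoom-in and zoom-out flags.
; Left-hand grab and both pinch states are recorded but not used here.
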(event `Key|LeapRightGrab`
  (params (Key :type "Key Structure" :default "LeapLeftPinch"))
  (:`Pressed`
    (set `self.IsGrabingRightHand` true))
  (:`Released`
    (set `self.IsGrabingRightHand` false)))

(event `Key|LeapLeftGrab`
  (params (Key :type "Key Structure" :default "LeapLeftPinch"))
  (:`Pressed`
    (set `self.IsGrabingLeftHand` true))
  (:`Released`
    (set `self.IsGrabingLeftHand` false)))

(event `self.ReceiveTick`
  (params (DeltaSeconds :type "Float (single-precision)"))
  (bind _citymap (`self.CityMap`))
  (`|ExecutionSequence`
    (:`then_0`
      (set `self.LeftHandPosition` (`SceneComponent.GetSocketLocation` (`/LeapMotion/Blueprints/Rigging/FloatingHands/LeapRiggedEchoHandsActor.LeftHandMesh` (`self.Hands`)) "lf_middle_meta")))
    (:`then_1`
      (set `self.RightHandPosition` (`SceneComponent.GetSocketLocation` (`/LeapMotion/Blueprints/Rigging/FloatingHands/LeapRiggedEchoHandsActor.RightHandMesh` (`self.Hands`)) "rt_middle_meta")))
    (:`then_2`
      (if (`self.IsGrabingRightHand`)
        (set `CityMap.CurrentGrabPosition` (`self.RightHandPosition`) _citymap)
        (else
          (set `CityMap.CurrentGrabPosition` (0.0 0.0 0.0) _citymap))))))

(event `Key|LeapLeftPinch`
  (params (Key :type "Key Structure" :default "LeapLeftPinch"))
  (:`Pressed`
    (set `self.IsPinchingLeftHand` true))
  (:`Released`
    (set `self.IsPinchingLeftHand` false)))

(event `Key|LeapRightPinch`
  (params (Key :type "Key Structure" :default "LeapLeftPinch"))
  (:`Pressed`
    (set `self.IsPinchingRightHand` true))
  (:`Released`
    (set `self.IsPinchingRightHand` false)))

(event `Key|Add`
  (params (Key :type "Key Structure" :default "LeapLeftPinch"))
  (bind _citymap (`self.CityMap`))
  (:`Pressed`
    (set `CityMap.ZoomIn` true _citymap))
  (:`Released`
    (set `CityMap.ZoomIn` false _citymap)))

(event `self.ReceiveBeginPlay`)

(event `Key|Subtract`
  (params (Key :type "Key Structure" :default "LeapLeftPinch"))
  (bind _citymap (`self.CityMap`))
  (:`Pressed`
    (set `CityMap.ZoomOut` true _citymap))
  (:`Released`
    (set `CityMap.ZoomOut` false _citymap)))

(fn `GetCamera`
  (returns (`Camera Component` :type "CameraComponent Object Reference"))
  (return null))

(fn `UserConstructionScript`)