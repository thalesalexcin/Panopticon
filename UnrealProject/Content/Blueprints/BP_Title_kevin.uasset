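; BP_Title_kevin plays a timed visual tutorial of hand gestures, starting when Starting_tuto is destroyed.
; A single linear chain of visibility toggles and fixed Delays shows the grab, zoom, rotate and finger-point visuals one after another.
; It ends by briefly showing a left/right hand choice with the Paneu element and signal / don't-signal text sprites, then hiding them all.
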(event `self.Starting_tuto.OnDestroyed`
  (bind _paneu (`self.Paneu`))
  (bind _text_dont_signal_sprite (`self.text_dont-signal_Sprite`))
  (bind _text_signal_sprite (`self.text_signal_Sprite`))
  (bind _fb_grabhand (`self.FB_GrabHand`))
  (bind _fb_handzoom (`self.FB_HandZoom`))
  (bind _fb_fingerpoint (`self.FB_FingerPoint`))
  (bind _fb_choicelefth (`self.FB_ChoiceLeftH`))
  (bind _fb_choicerighth (`self.FB_ChoiceRightH`))
  (bind _fb_handrotate (`self.FB_HandRotate`))
  (`SceneComponent.SetVisibility` _fb_grabhand true false)
  (`KismetSystemLibrary.Delay` 10.0)
  (`SceneComponent.SetVisibility` _fb_grabhand false false)
  (`SceneComponent.SetVisibility` _fb_handzoom true false)
  (`KismetSystemLibrary.Delay` 10.0)
  (`SceneComponent.SetVisibility` _fb_handzoom false false)
  (`SceneComponent.SetVisibility` _fb_handrotate true false)
  (`KismetSystemLibrary.Delay` 10.0)
  (`SceneComponent.SetVisibility` _fb_handrotate false false)
  (`SceneComponent.SetVisibility` _fb_fingerpoint true false)
  (`KismetSystemLibrary.Delay` 10.0)
  (`SceneComponent.SetVisibility` _fb_fingerpoint false false)
  (`SceneComponent.SetVisibility` _fb_choicerighth true false)
  (`SceneComponent.SetVisibility` _paneu true false)
  (`SceneComponent.SetVisibility` _text_dont_signal_sprite true false)
  (`SceneComponent.SetVisibility` _text_signal_sprite true false)
  (`SceneComponent.SetVisibility` _fb_choicelefth true false)
  (`KismetSystemLibrary.Delay` 10.0)
  (`SceneComponent.SetVisibility` _fb_choicerighth false false)
  (`SceneComponent.SetVisibility` _paneu false false)
  (`SceneComponent.SetVisibility` _text_dont_signal_sprite false false)
  (`SceneComponent.SetVisibility` _text_signal_sprite false false)
  (`SceneComponent.SetVisibility` _fb_choicelefth false false))

(fn `UserConstructionScript`)