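; BP_TriggersSelection colors the hand meshes as feedback when they overlap its left and right selection triggers during one specific game state.
; Each Tick it reads the PanoGameMode state, then shows a "not OK" material for the left hand in Left and an "OK" material for the right hand in Right.
; Otherwise the hands use the default material.
; A helper function sets a material only when it differs from the current one.
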(event `self.ReceiveTick`
  (params (DeltaSeconds :type "Float (single-precision)"))
  (bind _hands (`self.Hands`))
  (bind _lefthandmesh (`/LeapMotion/Blueprints/Rigging/FloatingHands/LeapRiggedEchoHandsActor.LeftHandMesh` _hands))
  (bind _righthandmesh (`/LeapMotion/Blueprints/Rigging/FloatingHands/LeapRiggedEchoHandsActor.RightHandMesh` _hands))
  (bind _aspano_game_mode (cast `/Game/Blueprints/PanoGameMode` (`GameplayStatics.GetGameMode`)))
  (if (`|EnumEquality` (`/Game/Blueprints/PanoGameMode.CurrentGameState` _aspano_game_mode) "NewEnumerator2")
    (`|ExecutionSequence`
      (:`then_0`
        ;[1 1 1] LeftHand
        (if (`PrimitiveComponent.IsOverlappingComponent` (`self.Left`) _lefthandmesh)
          (`self.SetCustomMaterial` _lefthandmesh "/Game/Materials/Hands/M_HandNotOk.M_HandNotOk")
          (else
            (`self.SetCustomMaterial` _lefthandmesh "/Game/Materials/Hands/M_Hands.M_Hands"))))
      (:`then_1`
        ;[1 1 1] RightHand
        (if (`PrimitiveComponent.IsOverlappingComponent` (`self.Right`) _righthandmesh)
          (`self.SetCustomMaterial` _righthandmesh "/Game/Materials/Hands/M_HandOk.M_HandOk")
          (else
            (`self.SetCustomMaterial` _righthandmesh "/Game/Materials/Hands/M_Hands.M_Hands")))))
    (else
      ;[1 1 1] Default
      (`|ExecutionSequence`
        (:`then_0`
          (`self.SetCustomMaterial` (`/LeapMotion/Blueprints/Rigging/FloatingHands/LeapRiggedEchoHandsActor.LeftHandMesh` _hands) "/Game/Materials/Hands/M_Hands.M_Hands"))
        (:`then_1`
          (`self.SetCustomMaterial` (`/LeapMotion/Blueprints/Rigging/FloatingHands/LeapRiggedEchoHandsActor.RightHandMesh` _hands) "/Game/Materials/Hands/M_Hands.M_Hands"))))))

(fn `SetCustomMaterial`
  (params (HandMesh :type "PrimitiveComponent Object Reference") (MatToSet :type "Material Object Reference"))
  (if (!= (`PrimitiveComponent.GetMaterial` HandMesh 0) MatToSet)
    (`PrimitiveComponent.SetMaterial` HandMesh 0 MatToSet))
  (return))

(fn `UserConstructionScript`)