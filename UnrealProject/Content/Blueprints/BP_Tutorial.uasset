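; Tutorial actor that teaches hand gestures and alert handling in the pano game.
; When its starting element is destroyed, it plays audio and shows timed hints for zoom, grab, rotate and alert, then spawns a tutorial alert near the camera, linked back to itself.
; Tick polls two flags to show signal/don't-signal choices, then hide them, change the game mode's state and destroy itself.
; Debug mode skips straight to that ending.
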(event `self.Starting_tuto.OnDestroyed`
  (bind _returnvalue (`KismetMathLibrary.Conv_IntToDouble` 4))
  (bind _fb_grabhand (`self.FB_GrabHand`))
  (bind _fb_handzoom (`self.FB_HandZoom`))
  (bind _fb_handrotate (`self.FB_HandRotate`))
  (if (`self.IsDebug`)
    (bind _aspano_game_mode (cast `/Game/Blueprints/PanoGameMode` (`GameplayStatics.GetGameMode`) :!label _label))
    (set `/Game/Blueprints/PanoGameMode.CurrentGameState` "NewEnumerator1" _aspano_game_mode)
    (`self.K2_DestroyActor` self)
    (else
      (`AkGameplayStatics.PostEvent` "/Game/WwiseAudio/Start.Start" self true)
      (`SceneComponent.SetVisibility` _fb_handzoom true false)
      (`KismetSystemLibrary.Delay` _returnvalue)
      (`SceneComponent.SetVisibility` _fb_handzoom false false)
      (`SceneComponent.SetVisibility` _fb_grabhand true false)
      (`KismetSystemLibrary.Delay` _returnvalue)
      (`SceneComponent.SetVisibility` _fb_grabhand false false)
      (`SceneComponent.SetVisibility` _fb_handrotate true false)
      (`KismetSystemLibrary.Delay` _returnvalue)
      (`SceneComponent.SetVisibility` _fb_handrotate false false)
      (`SceneComponent.SetVisibility` (`self.FB_hand_alert`) true false)
      (`KismetSystemLibrary.Delay` _returnvalue)
      ;[1 1 1] Spawn Alert
      (`self.SpawnAlertBubble`))))

(event `self.ReceiveTick`
  (params (DeltaSeconds :type "Float (single-precision)"))
  (bind _text_dont_signal_sprite (`self.text_dont-signal_Sprite`))
  (bind _text_signal_sprite (`self.text_signal_Sprite`))
  (bind _fb_choicelefth (`self.FB_ChoiceLeftH`))
  (bind _fb_choicerighth (`self.FB_ChoiceRightH`))
  (`|ExecutionSequence`
    (:`then_0`
      (if (`self.GoToDeciding`)
        (`SceneComponent.SetVisibility` (`self.FB_hand_alert`) false false)
        (`SceneComponent.SetVisibility` _fb_choicerighth true false)
        (`SceneComponent.SetVisibility` _text_dont_signal_sprite true false)
        (`SceneComponent.SetVisibility` _text_signal_sprite true false)
        (`SceneComponent.SetVisibility` _fb_choicelefth true false)))
    (:`then_1`
      (if (`self.GoToPop`)
        (`SceneComponent.SetVisibility` _fb_choicerighth false false)
        (`SceneComponent.SetVisibility` _text_dont_signal_sprite false false)
        (`SceneComponent.SetVisibility` _text_signal_sprite false false)
        (`SceneComponent.SetVisibility` _fb_choicelefth false false)
        (goto _label)))))

(fn `SpawnAlertBubble`
  (bind _returnvalue (`|SpawnActorFromClass` "/Game/Blueprints/BP_AlertActor_Tutorial.BP_AlertActor_Tutorial_C" (`KismetMathLibrary.MakeTransform` (+ (`PlayerCameraManager.GetCameraLocation` (`GameplayStatics.GetPlayerCameraManager` 0)) (50.0 0.0 -20.0))) "Undefined" "OverrideRootScale"))
  (set `/Game/Blueprints/BP_AlertActor_Tutorial.Hands` (`self.Hands`) _returnvalue)
  (set `/Game/Blueprints/BP_AlertActor_Tutorial.TutorialActor` self _returnvalue)
  (return))

(fn `UserConstructionScript`)