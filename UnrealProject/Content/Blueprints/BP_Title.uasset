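; BP_Title is the title screen actor, which advances the game state once both Leap Motion hands are held in place.
; BeginPlay posts the Panopticon Wwise event and sets the title state on PanoGameMode.
; Tick checks each hand mesh against its trigger, swaps that side's eye logo for a loading visual and accumulates hold time, resetting on exit.
; When both timers reach three seconds, it changes the state and destroys itself.
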(event `self.ReceiveBeginPlay`
  (`AkGameplayStatics.PostEvent` "/Game/WwiseAudio/Panopticon.Panopticon" self true)
  (bind _aspano_game_mode (cast `/Game/Blueprints/PanoGameMode` (`GameplayStatics.GetGameMode`)))
  (set `/Game/Blueprints/PanoGameMode.CurrentGameState` "NewEnumerator1" _aspano_game_mode))

(event `self.ReceiveTick`
  (params (DeltaSeconds :type "Float (single-precision)"))
  (bind _loadlogoleft (`self.LoadLogoLEFT`))
  (bind _loadlogoright (`self.LoadLogoRIGHT`))
  (`|ExecutionSequence`
    (:`then_0`
      ;[1 1 1] change logo right to loading
      (if (`PrimitiveComponent.IsOverlappingComponent` (`self.Tr_R`) (`/LeapMotion/Blueprints/Rigging/FloatingHands/LeapRiggedEchoHandsActor.RightHandMesh` (`self.LeapHands`)))
        (set `self.TimeRIght` (+ (`self.TimeRIght`) DeltaSeconds))
        (if (not _loadlogoright)
          (`SceneComponent.SetVisibility` (`self.EyeLogo_R`) false false)
          (`SceneComponent.SetVisibility` (`self.FB_Loading_R`) true false)
          (set `self.LoadLogoRIGHT` true))
        (elif _loadlogoright
          (set `self.TimeRIght` 0.0)
          (`SceneComponent.SetVisibility` (`self.FB_Loading_R`) false false)
          (`SceneComponent.SetVisibility` (`self.EyeLogo_R`) true false)
          (set `self.LoadLogoRIGHT` false))))
    (:`then_1`
      ;[1 1 1] start/stop logo left to loading
      (if (`PrimitiveComponent.IsOverlappingComponent` (`self.Tr_L`) (`/LeapMotion/Blueprints/Rigging/FloatingHands/LeapRiggedEchoHandsActor.LeftHandMesh` (`self.LeapHands`)))
        (set `self.TimeLeft` (+ (`self.TimeLeft`) DeltaSeconds))
        (if (not _loadlogoleft)
          (`SceneComponent.SetVisibility` (`self.EyeLogo_L`) false false)
          (`SceneComponent.SetVisibility` (`self.FB_Loading_L`) true false)
          (set `self.LoadLogoLEFT` true))
        (elif _loadlogoleft
          (set `self.TimeLeft` 0.0)
          (`SceneComponent.SetVisibility` (`self.FB_Loading_L`) false false)
          (`SceneComponent.SetVisibility` (`self.EyeLogo_L`) true false)
          (set `self.LoadLogoLEFT` false))))
    (:`then_2`
      (if (and (>= (`self.TimeLeft`) 3.0) (>= (`self.TimeRIght`) 3.0))
        (set `/Game/Blueprints/PanoGameMode.CurrentGameState` "NewEnumerator5" (stale `self.ReceiveBeginPlay` _aspano_game_mode))
        (`self.K2_DestroyActor`)))))

(fn `UserConstructionScript`)